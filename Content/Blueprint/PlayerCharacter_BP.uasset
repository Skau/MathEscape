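; Player character Blueprint that creates the in-game HUD and opens the pause menu.
; On BeginPlay it creates the HUD widget, stores a reference and adds it to the viewport.
; P or Escape, when the game is not paused, creates and shows a PauseMenu widget, pauses the game, switches to UI-only input and shows the mouse cursor.
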(event `Key|P`
  (params (Key :type "Key Structure"))
  (bind _returnvalue (`GameplayStatics.GetPlayerController` 0))
  (:`Pressed`
    (if (not (`GameplayStatics.IsGamePaused`)) :!label _label
      (bind _returnvalue_2 (`|CreateWidget` "/Game/Blueprint/HUD/PauseMenu.PauseMenu_C"))
      (bind _output_get (set `self.Pause Menu Reference` _returnvalue_2))
      (`UserWidget.AddToViewport` _output_get 0)
      (`GameplayStatics.SetGamePaused` true)
      (`WidgetBlueprintLibrary.SetInputMode_UIOnlyEx` _returnvalue)
      (set `PlayerController.bShowMouseCursor` true _returnvalue))))

(event `Key|Escape`
  (params (Key :type "Key Structure"))
  (:`Pressed`
    (goto _label)))

(event `self.ReceiveBeginPlay`
  (bind _returnvalue (`|CreateWidget` "/Game/Blueprint/HUD/HUD.HUD_C"))
  (bind _output_get (set `self.HUD Reference` _returnvalue))
  (`UserWidget.AddToViewport` _output_get 0))

(fn `UserConstructionScript`)